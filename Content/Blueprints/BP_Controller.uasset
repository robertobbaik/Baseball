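; Player controller for a networked chat-based guessing game, linking Widget_ChatWindow to BP_ChatMode.
; After a short BeginPlay delay it finds the chat widget and binds its send-message and game-start events.
; Requests and messages go to the game mode; game start stores the user index and generates a random four-element answer.
; Broadcasts from other users are checked against that answer via TakeMessage, and the result is shown in the widget.
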(event `self.ReceiveBeginPlay`
  (if (not (`|EnumEquality` (`self.GetRemoteRole`) "ROLE_None"))
    (`KismetSystemLibrary.Delay` 0.5)
    (bind _foundwidgets (`WidgetBlueprintLibrary.GetAllWidgetsOfClass` "/Game/Widgets/Widget_ChatWindow.Widget_ChatWindow_C"))
    (bind _output_get (set `self.Widget` (`|GetArrayItem` _foundwidgets)))
    (bind _aswidget_chat_window (cast `/Game/Widgets/Widget_ChatWindow` _output_get))
    (`|ExecutionSequence`
      (:`then_0`
        (add `/Game/Widgets/Widget_ChatWindow.SetMessageToUserController` _aswidget_chat_window (`|CreateDelegate` :!event `OnSendMsgToServer`)))
      (:`then_1`
        (add `/Game/Widgets/Widget_ChatWindow.GameStart` _aswidget_chat_window (`|CreateDelegate` :!event `Req_GameStart`))))))

(event `OnLoginWithID`
  (params (UserId :type String))
  (`self.OnUserLogin` UserId)
  (set `self.UserId` UserId))

(event `GotBroadcast`
  (params (Msg :type String) (UserIndex :type Integer))
  (bind _returnvalue (== UserIndex (`self.UserIndex`)))
  (if (not _returnvalue)
    (bind _returnvalue_2 (`CppBPlib.TakeMessage` Msg (`self.Correct Answer`)))
    (bind _aswidget_chat_window (cast `/Game/Widgets/Widget_ChatWindow` (`self.Widget`)))
    (`/Game/Widgets/Widget_ChatWindow.SetAnswer` _aswidget_chat_window _returnvalue _returnvalue_2)))

(event `OnSendMsgToServer`
  (params (Msg :type String) (UserIndex :type Integer))
  (bind _asbp_chat_mode (cast `/Game/GameModes/BP_ChatMode` (`GameplayStatics.GetGameMode`)))
  (`/Game/GameModes/BP_ChatMode.GotMessageFromClient` _asbp_chat_mode Msg UserIndex))

(event `Res_GameStart`
  (params (UserIndex :type Integer))
  (set `self.UserIndex` UserIndex)
  (bind _returnvalue (`CppBPlib.GetRandomArray` 4))
  (bind _output_get (set `self.Correct Answer` _returnvalue))
  (bind _returnvalue_2 (`CppBPlib.GetRandomArrayToString` _output_get))
  (bind _aswidget_chat_window (cast `/Game/Widgets/Widget_ChatWindow` (`self.Widget`)))
  (`/Game/Widgets/Widget_ChatWindow.ReceiveGameStart` _aswidget_chat_window (`self.UserIndex`) _returnvalue_2))

(event `Req_GameStart`
  (bind _asbp_chat_mode (cast `/Game/GameModes/BP_ChatMode` (`GameplayStatics.GetGameMode`)))
  (`/Game/GameModes/BP_ChatMode.GameStart_Event` _asbp_chat_mode))

(event `Test_Event`
  (params (TurnUserIndex :type Integer)))

(fn `IsServer`
  (returns (IsServer :type Boolean))
  (return (`KismetSystemLibrary.IsServer`)))

(fn `UserConstructionScript`)