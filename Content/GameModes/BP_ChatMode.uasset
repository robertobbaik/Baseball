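; BP_ChatMode is a game mode that relays chat and game-start events to player controllers.
; GotMessageFromClient forwards a message and sender index to each BP_Controller via GotBroadcast, while GameStart_Event calls ResGameStart on each with its array index.
; Turn_Event only prints a debug string.
; GetUserIndex increments and prints the UserIndex counter but always returns zero.
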(event `GotMessageFromClient`
  (params (Msg :type String) (UserIndex :type Integer))
  (bind _outactors (`GameplayStatics.GetAllActorsOfClass` "/Script/Engine.PlayerController"))
  (for _array_element _outactors
    (bind _asbp_controller (cast `/Game/Blueprints/BP_Controller` _array_element))
    (`/Game/Blueprints/BP_Controller.GotBroadcast` _asbp_controller Msg UserIndex)))

(event `GameStart_Event`
  (bind _outactors (`GameplayStatics.GetAllActorsOfClass` "/Script/Engine.PlayerController"))
  (for (_array_element _array_index) _outactors
    (bind _asbp_controller (cast `/Game/Blueprints/BP_Controller` _array_element))
    (`/Game/Blueprints/BP_Controller.Res_GameStart` _asbp_controller _array_index)))

(event `Turn_Event`
  (params (BP_Controller :type "/Game/Blueprints/BP_Controller Object Reference"))
  (`KismetSystemLibrary.PrintString` "Event_Turn"))

(fn `GetUserIndex`
  (returns (UserIndex :type Integer))
  (`KismetSystemLibrary.PrintString` (`KismetStringLibrary.Conv_IntToString` (`self.UserIndex`)))
  (bind _result (`/Engine/EditorBlueprintResources/StandardMacros.IncrementInt` (`self.UserIndex`))
    (:`  `
      (bind _output_get (set `self.UserIndex` _result))
      (`KismetSystemLibrary.PrintString` (`KismetStringLibrary.Conv_IntToString` _output_get))
      (return 0))))

(fn `UserConstructionScript`)